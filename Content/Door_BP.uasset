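; Interactive door Blueprint that swings open when an interaction begins and closes when it ends.
; A timeline drives the yaw of the Scene component, playing to open and reversing to close.
; A text prompt shows while the door is ready for interaction, hides during it, and turns to face the interacting pawn's camera on each ready tick.
; Each interaction event also prints a debug message.
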(event Custom|OpenDoor
  (bind _newtrack_0 (Timeline|Timeline_0 Play)
    (:Update
      (Transformation|SetRelativeRotation (Variables|Default|GetScene) (Math|Rotator|MakeRotator 0.0 0.0 _newtrack_0) false false))))

(event Custom|CloseDoor
  (bind _newtrack_0 (Timeline|Timeline_0 Reverse)
    (:Update
      (Transformation|SetRelativeRotation (Variables|Default|GetScene) (Math|Rotator|MakeRotator 0.0 0.0 _newtrack_0) false false))))

(event EventTickReadyInterative
  (params (Actor :type Actor%20Object%20Reference) (DeltaTime :type Float%20%28single-precision%29))
  (bind _aspawn (Utilities|Casting|CastToPawn Actor))
  (bind _returnvalue (Pawn|GetController _aspawn))
  (bind _aspc_bp (Utilities|Casting|CastToPC_BP _returnvalue))
  (bind _playercameramanager (Variables|/Script/Engine.PlayerController|GetPlayerCameraManager _aspc_bp))
  (bind _returnvalue_2 (Camera|GetCameraRotation _playercameramanager))
  (Transformation|SetWorldRotation (Variables|Default|GetTextRender) (Math|Rotator|MakeRotator (.roll _returnvalue_2) (* (.pitch _returnvalue_2) -1.0) (+ (.yaw _returnvalue_2) 1.8e+02)) false false)
  (Development|PrintString "Tick Ready" true false "(R=0.000000,G=0.660000,B=1.000000,A=1.000000)" 0.0))

(event EventTickInterative
  (params (Actor :type Actor%20Object%20Reference) (DeltaTime :type Float%20%28single-precision%29))
  (Development|PrintString "Tick" true true "(R=0.000000,G=0.660000,B=1.000000,A=1.000000)" 0.0))

(event EventEndReadyInterative
  (params (Actor :type Actor%20Object%20Reference))
  (Rendering|SetVisibility (Variables|Default|GetTextRender) false false)
  (Development|PrintString "End Ready" true false "(R=0.000000,G=0.660000,B=1.000000,A=1.000000)" 5.0))

(event EventEndInterative
  (params (Actor :type Actor%20Object%20Reference))
  (Rendering|SetVisibility (Variables|Default|GetTextRender) true false)
  (CallFunction|CloseDoor)
  (Development|PrintString "End" true false "(R=0.000000,G=0.660000,B=1.000000,A=1.000000)" 5.0))

(event EventBeginReadyInterative
  (params (Actor :type Actor%20Object%20Reference))
  (Rendering|SetVisibility (Variables|Default|GetTextRender) true false)
  (Development|PrintString "Begin Ready" true false "(R=0.000000,G=0.660000,B=1.000000,A=1.000000)" 5.0))

(event EventBeginInterative
  (params (Actor :type Actor%20Object%20Reference))
  (Rendering|SetVisibility (Variables|Default|GetTextRender) false false)
  (CallFunction|OpenDoor)
  (Development|PrintString "Begin" true false "(R=0.000000,G=0.660000,B=1.000000,A=1.000000)" 5.0))

(fn ConstructionScript)